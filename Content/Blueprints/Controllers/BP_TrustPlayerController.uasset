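; Player controller that owns the inventory UI and offers debug printouts of the player character's items.
; It creates WBP_Inventory on BeginPlay, and the OpenInventory input action toggles it on and off the viewport through a FlipFlop.
; The I key prints equipped item names from BP_TrustCharacter.
; An inventory-with-quantities printout and input-mode and focus switching exist but are never run.
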(event `self.ReceiveBeginPlay`
  (bind _returnvalue (`|CreateWidget` "/Game/Blueprints/UI/Inventory/WBP_Inventory.WBP_Inventory_C" self))
  (set `self.Inventory` _returnvalue))

(event `OpenInventory`
  (bind _inventory (`self.Inventory`))
  (`/Engine/EditorBlueprintResources/StandardMacros.IsValid` (`self.Inventory`)
    (:`Is Valid`
      (`/Engine/EditorBlueprintResources/StandardMacros.FlipFlop`
        (:`A`
          (`UserWidget.AddToViewport` _inventory 0))
        (:`B`
          (`Widget.RemoveFromParent` _inventory))))))

(event `InputAction|OpenInventory`
  (params (Key :type "Key Structure"))
  (:`Pressed`
    (`self.OpenInventory`)))

(event `Key|I`
  (params (Key :type "Key Structure"))
  (:`Pressed`
    (`self.GetEquippedItems`)))

(event `GetInventory`
  (bind _asbp_trust_character (cast `/Game/Blueprints/Characters/BP_TrustCharacter` (`GameplayStatics.GetPlayerPawn` 0)))
  (for _array_element (`InventoryComponent.GetInventoryItems` (`TrustCharacter.PlayerInventory` _asbp_trust_character))
    (`KismetSystemLibrary.PrintString` (`KismetStringLibrary.Concat_StrStr` (`KismetTextLibrary.Conv_TextToString` (`Item.ItemDisplayName` _array_element)) "[" (`KismetStringLibrary.Conv_IntToString` (`Item.GetQuantity` _array_element)) "]"))))

(event `GetEquippedItems`
  (bind _asbp_trust_character (cast `/Game/Blueprints/Characters/BP_TrustCharacter` (`GameplayStatics.GetPlayerPawn` 0)))
  (bind _values (`BlueprintMapLibrary.Map_Values` (`TrustCharacter.GetEquippedItems` _asbp_trust_character)))
  (for _array_element _values
    (`KismetSystemLibrary.PrintString` (`KismetTextLibrary.Conv_TextToString` (`Item.ItemDisplayName` _array_element)))))

(fn `UserConstructionScript`)